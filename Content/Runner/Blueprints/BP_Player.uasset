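; Player pawn for a three-lane endless runner with keyboard and swipe input for lane changes, turns, jumps and slides.
; A 0.02-second timer advances distance and score, periodically raising speed and global time dilation.
; Tick moves the capsule's XY along the main or curve-floor spline while interpolating the mesh toward lane markers and heading.
; Floor overlaps trigger spawning and destroy older floors; Lose resets dilation and shows the death menu.
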(event `Init Location`
  (`self.Move Along Spline` (`/Game/Runner/Blueprints/BP_Spline.Spline` (`self.BP_Spline`))))

(event `self.ReceiveBeginPlay`
  (set `self.Location Points` (`|MakeArray` (`self.Sphere`) (`self.Sphere1`) (`self.Sphere2`)))
  (bind _returnvalue (`|CreateWidget` "/Game/Runner/Widgets/W_HUD.W_HUD_C" (`GameplayStatics.GetPlayerController` 0)))
  (set `/Game/Runner/Widgets/W_HUD.Player ref` self _returnvalue)
  (`UserWidget.AddToViewport` _returnvalue 0)
  (bind _returnvalue_2 (`|CreateWidget` "/Game/Runner/Widgets/W_Counter.W_Counter_C" (`GameplayStatics.GetPlayerController` 0)))
  (`UserWidget.AddToViewport` _returnvalue_2 0)
  (set `self.Speed` 0.0)
  (set `self.Init Rotation` (`SceneComponent.K2_GetComponentRotation` (`self.Mesh`))))

(event `StartGame`
  (set `self.Start Game` true)
  (`self.Changes Values`)
  (set `self.Speed` 30.0))

(event `Changes Values`
  (bind _point (`self.Point`))
  (if (and (not (`self.End Game`)) (`self.Start Game`))
    (set `self.Curve Distance` (+ (`self.Curve Distance`) (`self.Speed`)))
    (set `self.Distance` (+ (`self.Distance`) (`self.Speed`)))
    (`/Engine/EditorBlueprintResources/StandardMacros.IncrementInt` _point
      (:`  `
        (if (== (mod _point 1000) 0)
          (bind _output_get (set `self.Time Dilation` (+ (`self.Time Dilation`) 0.1)))
          (`GameplayStatics.SetGlobalTimeDilation` _output_get)
          (set `self.Speed` (+ (`self.Speed`) 3.0)))
        (`KismetSystemLibrary.K2_SetTimerDelegate` (delegate `Changes Values`) 0.02)))))

(event `self.CapsuleComponent.OnComponentBeginOverlap`
  (params (OverlappedComponent :type "PrimitiveComponent Object Reference") (OtherActor :type "Actor Object Reference") (OtherComp :type "PrimitiveComponent Object Reference") (OtherBodyIndex :type Integer) (bFromSweep :type Boolean) (SweepResult :type "HitResult Structure (by ref)"))
  (bind _asbp_floor (cast `/Game/Runner/Blueprints/Floors/BP_Floor` OtherActor))
  (if (!= _asbp_floor (`self.New Floor`))
    (`/Engine/EditorBlueprintResources/StandardMacros.IsValid` (`self.Last floor`)
      (:`Is Valid`
        (`self.K2_DestroyActor` (`self.Last floor`)))
      (:`Is Not Valid`
        _))
    (set `self.Last floor` (`self.New Floor`))
    (bind _output_get (set `self.New Floor` _asbp_floor))
    (set `self.In Curve` (`/Game/Runner/Blueprints/Floors/BP_Floor.Is Curve ?` _output_get))
    (`SplineComponent.SetLocationAtSplinePoint` (`/Game/Runner/Blueprints/Floors/BP_Floor.Curve Spline` _output_get) 0 (`SceneComponent.K2_GetComponentLocation` (`self.CapsuleComponent`)) "World" true)
    (`/Game/Runner/Blueprints/BP_Floor_Generator.Spawn Floor` (`self.BP_FloorSpawner`) true)))

(event `self.ReceiveTick`
  (params (DeltaSeconds :type "Float (single-precision)"))
  (bind _mesh (`self.Mesh`))
  (bind _mesh_2 (`self.Mesh`))
  (bind (_init_rotation_roll _init_rotation_pitch _init_rotation_yaw) (`KismetMathLibrary.BreakRotator` (`self.Init Rotation`)))
  (bind (_returnvalue_x _returnvalue_y _returnvalue_z) (`KismetMathLibrary.BreakVector` (`SceneComponent.K2_GetComponentLocation` _mesh)))
  (bind (_returnvalue_x_2 _returnvalue_y_2) (`KismetMathLibrary.BreakVector` (`SceneComponent.K2_GetComponentLocation` (`|GetArrayItem` (`self.Location Points`) (`self.Actual side`)))))
  (if (and (not (`self.End Game`)) (`self.Start Game`))
    (`SceneComponent.K2_SetWorldRotation` _mesh_2 (`KismetMathLibrary.RInterpTo` (`SceneComponent.K2_GetComponentRotation` _mesh_2) (`KismetMathLibrary.MakeRotator` _init_rotation_roll _init_rotation_pitch (+ _init_rotation_yaw (`self.Rotation Offset`))) DeltaSeconds 5.0) false false)
    (`SceneComponent.K2_SetWorldRotation` (`self.Sphere3`) (`KismetMathLibrary.MakeRotator` 0.0 0.0 (`self.Rotation Offset`)) false false)
    (if (`self.In Curve`)
      (`self.Move Along Spline` (`/Game/Runner/Blueprints/Floors/BP_Floor.Curve Spline` (`self.New Floor`)) (`self.Curve Distance`))
      (else
        (set `self.Curve Distance` 0.0)
        (`self.Move Along Spline` (`/Game/Runner/Blueprints/BP_Spline.Spline` (`self.BP_Spline`)) (`self.Distance`))))
    (`SceneComponent.K2_SetWorldLocation` _mesh (`KismetMathLibrary.MakeVector` (`KismetMathLibrary.FInterpTo` _returnvalue_x _returnvalue_x_2 DeltaSeconds 5.0) (`KismetMathLibrary.FInterpTo` _returnvalue_y _returnvalue_y_2 DeltaSeconds 5.0) _returnvalue_z) false false)))

(event `Key|A`
  (params (Key :type "Key Structure"))
  (:`Pressed`
    (if (and (not (`self.End Game`)) (`self.Start Game`)) :!label _label
      (if (`self.In Curve`)
        (cast `/Game/Runner/Blueprints/Floors/BP_Left_Floor` (`self.New Floor`))
        (set `self.In Curve` false)
        (set `self.Rotation Offset` (+ (`self.Rotation Offset`) -90.0))
        (elif (> (`self.Actual side`) 0)
          (`/Engine/EditorBlueprintResources/StandardMacros.DecrementInt` (`self.Actual side`)))))))

(event `Move Left`
  (goto _label))

(event `Key|D`
  (params (Key :type "Key Structure"))
  (:`Pressed`
    (if (and (not (`self.End Game`)) (`self.Start Game`)) :!label _label_2
      (if (`self.In Curve`)
        (cast `/Game/Runner/Blueprints/Floors/BP_Right_Floor` (`self.New Floor`))
        (set `self.In Curve` false)
        (set `self.Rotation Offset` (+ (`self.Rotation Offset`) 90.0))
        (elif (< (`self.Actual side`) (- (`KismetArrayLibrary.Array_Length` (`self.Location Points`)) 1))
          (`/Engine/EditorBlueprintResources/StandardMacros.IncrementInt` (`self.Actual side`)))))))

(event `Move Right`
  (goto _label_2))

(event `Sliding`
  (bind _returnvalue (`SkeletalMeshComponent.GetAnimInstance` (`self.Mesh`)))
  (if (and (not (`self.End Game`)) (`self.Start Game`)) :!label _label_3
    (message `/Game/Runner/Blueprint_Interfaces/BPI_Player.Slide` _returnvalue true)
    (set `self.Is Slide` true)
    (`KismetSystemLibrary.RetriggerableDelay` 0.5)
    (message `/Game/Runner/Blueprint_Interfaces/BPI_Player.Slide` _returnvalue false)
    (set `self.Is Slide` false)))

(event `Key|LeftAlt`
  (params (Key :type "Key Structure"))
  (:`Pressed`
    (goto _label_3)))

(event `Key|SpaceBar`
  (params (Key :type "Key Structure"))
  (:`Pressed`
    (if (and (not (`self.End Game`)) (`self.Start Game`)) :!label _label_4
      (`self.Jump`))))

(event `Jumping`
  (goto _label_4))

(event `Lose`
  (set `self.End Game` true)
  (`GameplayStatics.SetGlobalTimeDilation` 1.0)
  (message `/Game/Runner/Blueprint_Interfaces/BPI_Player.Die` (`SkeletalMeshComponent.GetAnimInstance` (`self.Mesh`)))
  (`KismetSystemLibrary.Delay` 2.0)
  (bind _returnvalue (`|CreateWidget` "/Game/Runner/Widgets/W_DieMenu.W_DieMenu_C" (`GameplayStatics.GetPlayerController` 0)))
  (set `/Game/Runner/Widgets/W_DieMenu.Player ref` self _returnvalue)
  (`UserWidget.AddToViewport` _returnvalue 0))

(event `Add Point`
  (params (B :type Integer))
  (set `self.Point` (+ (`self.Point`) B)))

(event `InputTouch`
  (params (Location :type "Vector Structure") (FingerIndex :type "ETouchIndex Enum"))
  (bind _x (.x Location))
  (bind _y (.y Location))
  (bind (_returnvalue_x _returnvalue_y) (`KismetMathLibrary.BreakVector2D` (- (`self.Start touch`) (`self.End touch`))))
  (:`Pressed`
    (set `self.Start touch` (`KismetMathLibrary.MakeVector2D` _x _y)))
  (:`Released`
    (set `self.End touch` (`KismetMathLibrary.MakeVector2D` _x _y))
    (`|ExecutionSequence`
      (:`then_0`
        (if (> _returnvalue_x 100.0)
          (`self.Move Left`)))
      (:`then_1`
        (if (< _returnvalue_x -100.0)
          (`self.Move Right`)))
      (:`then_2`
        (if (> _returnvalue_y 100.0)
          (`self.Jumping`)))
      (:`then_3`
        (if (< _returnvalue_y -100.0)
          (`self.Sliding`))))))

(fn `UserConstructionScript`)