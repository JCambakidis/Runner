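; BP_Floor is a floor piece for the runner game, built around a spline path and a BoxForPlayer component.
; The construction script moves BoxForPlayer to the spline's first point.
; AddCoinOnSpline spawns coins as child actor components and teleports them to evenly spaced distances along a given spline.
; The event graph holds no logic, and nothing in this Blueprint calls AddCoinOnSpline.
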(fn `Add Coin On Spline`
  (params (`Number Of Coins` :type Integer) (Spline :type "SplineComponent Object Reference"))
  (locals (NewLocalVar_0 :type "Float (double-precision)" :default 1.0))
  (for _index (range (+ `Number Of Coins` 1))
    (bind _returnvalue (`AddComponent|NODE_AddChildActorComponent-0` :`RelativeTransform` (`KismetMathLibrary.MakeTransform` (0.0 0.0 230.0))))
    (`SceneComponent.K2_SetWorldLocation` _returnvalue (`SplineComponent.GetLocationAtDistanceAlongSpline` Spline (* (/ (`SplineComponent.GetSplineLength` Spline) (`KismetMathLibrary.Conv_IntToDouble` `Number Of Coins`)) (`KismetMathLibrary.Conv_IntToDouble` _index)) "World") false true)))

(fn `UserConstructionScript`
  (`SceneComponent.K2_SetWorldLocation` (`self.Box For player`) (`SplineComponent.GetLocationAtSplinePoint` (`self.Spline`) 0 "World") false false))