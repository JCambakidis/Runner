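; Floor generator for a runner game that builds the track at BeginPlay from a seed floor created in the construction script, then places the player on it.
; SpawnFloor snaps each piece to the previous one's Front, Right or Left socket and feeds it into BPSpline.
; Turns are random but spaced by a run of straight pieces, and the opening pieces have their obstacles cleared.
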(event `Spawn Floor`
  (params (`With Obstacle ?` :type Boolean))
  (bind _spawnedfloor (`self.SpawnedFloor`))
  (bind _returnvalue (`KismetArrayLibrary.Array_Length` _spawnedfloor))
  (if (> (`self.Spawn Count`) 2)
    (set `self.TMP` (`KismetMathLibrary.RandomIntegerInRange` 0 2))
    (else
      (set `self.TMP` 0)))
  (bind _returnvalue_2 (`|SpawnActorFromClass` (`|GetArrayItem` (`self.FloorType`) (`self.TMP`)) (`KismetMathLibrary.MakeTransform` (0.0 0.0 0.0)) "Undefined" "OverrideRootScale" null null))
  (`KismetArrayLibrary.Array_Add` (`self.SpawnedFloor`) _returnvalue_2)
  (if (> (`self.TMP`) 0)
    (set `self.Spawn Count` 0)
    (else
      (`/Engine/EditorBlueprintResources/StandardMacros.IncrementInt` (`self.Spawn Count`)
        (:`  `
          _))))
  (if (> _returnvalue 0)
    (`self.K2_AttachToComponent` _returnvalue_2 (`/Game/Runner/Blueprints/Floors/BP_Floor.StaticMesh` (`|GetArrayItem` _spawnedfloor (- _returnvalue 2))) (select `int` (`self.TMP`) :`0` "Front" :`1` "Right" :`2` "Left" :!type "Name") "SnapToTarget" "SnapToTarget" "KeepRelative" true)
    (`/Game/Runner/Blueprints/BP_Spline.Add Spline Point` (`self.BP_Spline`) _returnvalue_2)
    (if (not `With Obstacle ?`)
      (bind _asbp_front_floor (cast `/Game/Runner/Blueprints/Floors/BP_Front_Floor` _returnvalue_2))
      (bind _obstacle (`/Game/Runner/Blueprints/Floors/BP_Front_Floor.Obstacle` _asbp_front_floor))
      (`/Engine/EditorBlueprintResources/StandardMacros.IsValid` _obstacle
        (:`Is Valid`
          (`StaticMeshComponent.SetStaticMesh` _obstacle null)
          (set `/Game/Runner/Blueprints/Floors/BP_Front_Floor.Obstacles Types` "NewEnumerator5" _asbp_front_floor))))))

(event `self.ReceiveBeginPlay`
  (for _index (range 11)
    (if (< _index 3)
      (`self.Spawn Floor` false)
      (else
        (`self.Spawn Floor` true))))
  (`SplineComponent.SetLocationAtSplinePoint` (`/Game/Runner/Blueprints/BP_Spline.Spline` (`self.BP_Spline`)) 0 (`SplineComponent.GetLocationAtSplinePoint` (`/Game/Runner/Blueprints/Floors/BP_Floor.Spline` (`|GetArrayItem` (`self.SpawnedFloor`) 1)) 0 "World") "World" true)
  (bind _outactors (`GameplayStatics.GetAllActorsOfClass` "/Game/Runner/Blueprints/BP_Player.BP_Player_C"))
  (bind _output (`|GetArrayItem` _outactors))
  (set `/Game/Runner/Blueprints/BP_Player.New Floor` (`|GetArrayItem` (`self.SpawnedFloor`)) _output)
  (`/Game/Runner/Blueprints/BP_Player.Init Location` _output))

(fn `UserConstructionScript`
  (bind _returnvalue (`AddComponent|NODE_AddChildActorComponent-0` :`bManualAttachment` true :`RelativeTransform` (`KismetMathLibrary.MakeTransform` (0.0 0.0 0.0))))
  (bind _asbp_floor (cast `/Game/Runner/Blueprints/Floors/BP_Floor` (`ChildActorComponent.ChildActor` _returnvalue)))
  (`KismetArrayLibrary.Array_Add` (`self.SpawnedFloor`) _asbp_floor))