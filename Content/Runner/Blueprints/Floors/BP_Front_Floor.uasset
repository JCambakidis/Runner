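; Forward floor segment for a runner game that spawns a random obstacle and optional coins, and decides when the player loses.
; The construction script rolls a lane box, jump block, slide block or nothing, attaches the mesh at its point, and may line coins along a lane spline, except on jump and slide segments.
; A single DieBox overlap calls Lose by checking the player's lane, falling or slide state against the obstacle type.
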(event `self.Die Box.OnComponentBeginOverlap`
  (params (OverlappedComponent :type "PrimitiveComponent Object Reference") (OtherActor :type "Actor Object Reference") (OtherComp :type "PrimitiveComponent Object Reference") (OtherBodyIndex :type Integer) (bFromSweep :type Boolean) (SweepResult :type "HitResult Structure (by ref)"))
  (bind _asbp_player (cast `/Game/Runner/Blueprints/BP_Player` OtherActor))
  (switch `/Game/Runner/Blueprints/Floors/E_Obstacles_Types` (`self.Obstacles Types`)
    (:`NewEnumerator0`
      (bind _actual_side (`/Game/Runner/Blueprints/BP_Player.Actual side` _asbp_player))
      (if (== _actual_side 2)
        (`/Game/Runner/Blueprints/BP_Player.Lose` _asbp_player :!label _label)))
    (:`NewEnumerator1`
      (if (== _actual_side 1)
        (goto _label)))
    (:`NewEnumerator2`
      (if (== _actual_side 0)
        (goto _label)))
    (:`NewEnumerator3`
      (if (not (`NavMovementComponent.IsFalling` (`Character.CharacterMovement` _asbp_player)))
        (goto _label)))
    (:`NewEnumerator4`
      (if (not (`/Game/Runner/Blueprints/BP_Player.Is Slide` _asbp_player))
        (goto _label)))))

(fn `UserConstructionScript`
  (bind _returnvalue (`KismetMathLibrary.RandomBool`))
  (bind _coins_spline1 (`self.Coins Spline1`))
  (bind _returnvalue_2 (`KismetMathLibrary.MakeVector` (`KismetMathLibrary.RandomFloatInRange` 0.5 1.0) (`KismetMathLibrary.RandomFloatInRange` 0.5 1.0) 1.0))
  (`parent.UserConstructionScript`)
  (set `self.Obstacles Types` (select `int` (`KismetMathLibrary.RandomIntegerInRange` 0 5) :`0` "NewEnumerator0" :`1` "NewEnumerator1" :`2` "NewEnumerator2" :`3` "NewEnumerator3" :`4` "NewEnumerator4" :`5` "NewEnumerator5" :!type "/Game/Runner/Blueprints/Floors/E_Obstacles_Types Enum"))
  (if (> (`KismetMathLibrary.RandomIntegerInRange` 0 100) 50)
    (set `self.Is Coin` true))
  (switch `/Game/Runner/Blueprints/Floors/E_Obstacles_Types` (`self.Obstacles Types`)
    (:`NewEnumerator0`
      (`self.Add Obstacle` (`self.BoxPoint`) "/Game/Platformer/Meshes/Pl_MetalBox_2m.Pl_MetalBox_2m" _returnvalue_2))
    (:`NewEnumerator1`
      (`self.Add Obstacle` (`self.BoxPoint1`) "/Game/Platformer/Meshes/Pl_MetalBox_2m.Pl_MetalBox_2m" _returnvalue_2))
    (:`NewEnumerator2`
      (`self.Add Obstacle` (`self.BoxPoint2`) "/Game/Platformer/Meshes/Pl_MetalBox_2m.Pl_MetalBox_2m" _returnvalue_2))
    (:`NewEnumerator3`
      (`self.Add Obstacle` (`self.JumpPoint`) "/Game/Platformer/Meshes/Beanstalks/Pl_StoneBlock_03.Pl_StoneBlock_03" (1.0 1.0 1.5)))
    (:`NewEnumerator4`
      (`self.Add Obstacle` (`self.SlidePoint`) "/Game/Platformer/Meshes/Beanstalks/Pl_StoneBlock_03.Pl_StoneBlock_03" (1.0 1.0 1.5)))
    (:`NewEnumerator5`
      _))
  (if (`self.Is Coin`)
    (switch `/Game/Runner/Blueprints/Floors/E_Obstacles_Types` (`self.Obstacles Types`)
      (:`NewEnumerator0`
        (if (`KismetMathLibrary.RandomBool`) :!label _label
          (`self.Add Coin On Spline` 5 (`self.Coins Spline`))
          (else
            (`self.Add Coin On Spline` 5 _coins_spline1))))
      (:`NewEnumerator1`
        (if _returnvalue :!label _label_2
          (`self.Add Coin On Spline` 5 _coins_spline1)
          (else
            (`self.Add Coin On Spline` 5 (`self.Coins Spline2`)))))
      (:`NewEnumerator2`
        (if (`KismetMathLibrary.RandomBool`)
          (`self.Add Coin On Spline` 5 (`self.Coins Spline2`))
          (else
            (`self.Add Coin On Spline` 5 (`self.Coins Spline`)))))
      (:`NewEnumerator5`
        (if _returnvalue
          (goto _label_2)
          (else
            (goto _label)))))))